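; Lobby player controller that shows the lobby widget to the local player and handles player selection and ready toggling.
; On BeginPlay it caches the game state and player state, retrying each tick until the latter is valid.
; Selection and ready changes pass through SERVER-to-CLIENT event chains that update the local controller's widget via the PlayerArray.
; Both record results in GameState arrays indexed by player name.
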(event Custom|SelectCLIENT
  (params (ButtonSelected :type String) (PlayerName :type Text))
  (Utilities|FlowControl|Sequence
    (:then_0
      (for _array_element (Variables|/Script/Engine.GameStateBase|GetPlayerArray (Variables|Default|GetGameState))
        (Utilities|IsValid (Game|GetPlayerController _array_element)
          (:Is%20Valid
            (if (Pawn|IsLocalController (Game|GetPlayerController _array_element))
              (bind _aspc_lobby (Utilities|Casting|CastToPC_Lobby (Game|GetPlayerController _array_element)))
              (Default|Select (Variables|PC_Lobby_C|GetWBP_Lobby _aspc_lobby) ButtonSelected PlayerName))))))
    (:then_1
      (CallFunction|UpdateSelection (Utilities|String|ToString(Text) PlayerName) ButtonSelected))))

(event Custom|Select
  (params (ButtonSelected :type String) (PlayerName :type Text))
  (CallFunction|SelectSERVER ButtonSelected PlayerName)
  (CallFunction|UpdateSelection (Utilities|String|ToString(Text) PlayerName) ButtonSelected))

(event Custom|UpdateSelection
  (params (PlayerName :type String%20%28by%20ref%29) (ButtonName :type String%20%28by%20ref%29))
  (bind _gamestate (Variables|Default|GetGameState))
  (Utilities|Array|SetArrayElem (Variables|/Game/Game/Blueprints/BP_GameState.BP_GameState_C|GetPlayerSelection _gamestate) (Utilities|Array|FindItem (Variables|/Game/Game/Blueprints/BP_GameState.BP_GameState_C|GetPlayerName _gamestate) PlayerName) ButtonName))

(event Custom|ToggleReadyCLIENT
  (params (Player :type String) (Ready :type Boolean))
  (bind _gamestate (Variables|Default|GetGameState))
  (bind _playername (Variables|/Game/Game/Blueprints/BP_GameState.BP_GameState_C|GetPlayerName _gamestate))
  (bind _returnvalue (Utilities|Array|FindItem _playername Player))
  (Utilities|FlowControl|Sequence
    (:then_0
      (for _array_element (Variables|/Script/Engine.GameStateBase|GetPlayerArray _gamestate)
        (Utilities|IsValid (Game|GetPlayerController _array_element)
          (:Is%20Valid
            (if (Pawn|IsLocalController (Game|GetPlayerController _array_element))
              (bind _aspc_lobby (Utilities|Casting|CastToPC_Lobby (Game|GetPlayerController _array_element)))
              (Default|ToggleReady (Variables|PC_Lobby_C|GetWBP_Lobby _aspc_lobby) (Utilities|Array|Get(acopy) (Variables|/Game/Game/Blueprints/BP_GameState.BP_GameState_C|GetPlayerSelection _gamestate) _returnvalue) Ready))))))
    (:then_1
      (Utilities|Array|SetArrayElem (Variables|/Game/Game/Blueprints/BP_GameState.BP_GameState_C|GetPlayerReady _gamestate) _returnvalue Ready))))

(event Custom|ToggleReadySERVER
  (params (Player :type String) (Ready :type Boolean))
  (CallFunction|ToggleReadyCLIENT Player Ready))

(event Custom|SelectSERVER
  (params (ButtonSelected :type String) (PlayerName :type Text))
  (CallFunction|SelectCLIENT ButtonSelected PlayerName))

(event EventBeginPlay
  (bind _self self)
  (bind _playerstate (Variables|GetPlayerState))
  (Utilities|FlowControl|Sequence
    (:then_0
      (Utilities|IsValid _playerstate :!label _label
        (:Is%20Valid
          (bind _asbp_ps_game (Utilities|Casting|CastToBP_PS_Game _playerstate))
          (Variables|Default|SetPlayState _asbp_ps_game))
        (:Is%20Not%20Valid
          (Utilities|FlowControl|DelayUntilNextTick)
          (goto _label))))
    (:then_1
      (bind _asbp_game_state (Utilities|Casting|CastToBP_GameState (Game|GetGameState)))
      (Variables|Default|SetGameState _asbp_game_state))
    (:then_2
      (if (Pawn|IsLocalController)
        (bind _returnvalue (UserInterface|CreateWidget "/Game/Game/Widgets/WBP_Lobby.WBP_Lobby_C" _self))
        (bind _output_get (Variables|Default|SetWBP_Lobby _returnvalue))
        (UserInterface|Viewport|AddtoViewport _output_get 0)
        (Variables|/Script/Engine.PlayerController|SetbShowMouseCursor _self true)))))

(fn ConstructionScript)