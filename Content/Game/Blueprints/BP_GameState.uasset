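; Lobby game state that tracks each player's button selection and ready status and starts the match.
; Tick registers players by Steam persona name, with an "Offline" fallback, into parallel name, selection and ready arrays, then server-travels to DefaultLevel once all ready flags are true.
; Selection and ready events pass through SERVER-to-CLIENT chains that update those arrays and the local PC_Lobby's lobby widget.
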(event Custom|SelectCLIENT
  (params (ButtonSelected :type String) (PlayerName :type Text))
  (Utilities|FlowControl|Sequence
    (:then_0
      (for _array_element (Variables|Default|GetPlayerArray)
        (Utilities|IsValid (Game|GetPlayerController _array_element)
          (:Is%20Valid
            (if (Pawn|IsLocalController (Game|GetPlayerController _array_element))
              (bind _aspc_lobby (Utilities|Casting|CastToPC_Lobby (Game|GetPlayerController _array_element)))
              (Default|Select (Variables|/Game/Game/Blueprints/PC_Lobby.PC_Lobby_C|GetWBP_Lobby _aspc_lobby) ButtonSelected PlayerName))))))
    (:then_1
      (CallFunction|UpdateSelection (Utilities|String|ToString(Text) PlayerName) ButtonSelected))))

(event Custom|Select
  (params (ButtonSelected :type String) (PlayerName :type Text))
  (CallFunction|SelectSERVER ButtonSelected PlayerName))

(event Custom|UpdateSelection
  (params (PlayerName :type String%20%28by%20ref%29) (ButtonName :type String%20%28by%20ref%29))
  (Utilities|Array|SetArrayElem (Variables|Default|GetPlayerSelection) (Utilities|Array|FindItem (Variables|Default|GetPlayerName) PlayerName) ButtonName))

(event Custom|ToggleReadyCLIENT
  (params (Player :type String) (Ready :type Boolean))
  (bind _playername (Variables|Default|GetPlayerName))
  (bind _returnvalue (Utilities|Array|FindItem _playername Player))
  (Utilities|FlowControl|Sequence
    (:then_0
      (for _array_element (Variables|Default|GetPlayerArray)
        (Utilities|IsValid (Game|GetPlayerController _array_element)
          (:Is%20Valid
            (if (Pawn|IsLocalController (Game|GetPlayerController _array_element))
              (bind _aspc_lobby (Utilities|Casting|CastToPC_Lobby (Game|GetPlayerController _array_element)))
              (Default|ToggleReady (Variables|/Game/Game/Blueprints/PC_Lobby.PC_Lobby_C|GetWBP_Lobby _aspc_lobby) (Utilities|Array|Get(acopy) (Variables|Default|GetPlayerSelection) _returnvalue) Ready))))))
    (:then_1
      (Utilities|Array|SetArrayElem (Variables|Default|GetPlayerReady) _returnvalue Ready))))

(event Custom|ToggleReadySERVER
  (params (Player :type String) (Ready :type Boolean))
  (CallFunction|ToggleReadyCLIENT Player Ready))

(event Custom|SelectSERVER
  (params (ButtonSelected :type String) (PlayerName :type Text))
  (CallFunction|SelectCLIENT ButtonSelected PlayerName))

(event EventBeginPlay)

(event EventTick
  (params (DeltaSeconds :type Float%20%28single-precision%29))
  (bind _playername (Variables|Default|GetPlayerName))
  (Utilities|FlowControl|Sequence
    (:then_0
      (for _array_element (Variables|Default|GetPlayerArray)
        (bind _returnvalue (Class|AdvancedSteamFriendsLibrary|GetSteamPersonaName (Class|AdvancedSessionsLibrary|GetUniqueNetIDfromPlayerState _array_element)))
        (if (not (Utilities|Array|ContainsItem _playername (Utilities|String|SelectString (Utilities|Array|Get(acopy) _playername) _returnvalue (Utilities|Enum|Equal(Enum) _returnvalue ""))))
          (Utilities|Array|Add (Variables|Default|GetPlayerReady) false)
          (Utilities|Array|Add (Variables|Default|GetPlayerSelection) "")
          (Utilities|Array|Add (Variables|Default|GetPlayerName) (Utilities|String|SelectString "Offline" _returnvalue (Utilities|Enum|Equal(Enum) _returnvalue ""))))))
    (:then_2
      (Variables|Default|SetLaunch true)
      (for _array_element_2 (Variables|Default|GetPlayerReady)
        (Variables|Default|SetLaunch (and _array_element_2 (Variables|Default|GetLaunch))))
      (if (Variables|Default|GetLaunch)
        (Utilities|FlowControl|DelayUntilNextTick)
        (Class|AdvancedSessionsLibrary|ServerTravel "DefaultLevel" false false)))))

(fn ConstructionScript)